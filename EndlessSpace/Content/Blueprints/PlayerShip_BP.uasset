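; Player ship that hops between positions on a 3x3 grid in its local Y-Z plane.
; Directional input presses step the MoveShipTo target one cell, limited to one either side of center.
; Each tick, MoveShip slides the Cube component toward that cell, with a separate vertical speed factor, and snaps when close.
; Touch press and release locations are stored but not used in this graph.
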(event Custom|MoveShip
  (params (Delta%20Seconds :type Float%20%28single-precision%29))
  (bind _moveshipto (Variables|Default|GetMoveShipTo))
  (bind _shiphorizontalmovement (Variables|Default|GetShipHorizontalMovement))
  (bind _shipverticalmovement (Variables|Default|GetShipVerticalMovement))
  (bind _cube (Variables|Default|GetCube))
  (bind _returnvalue (Transformation|GetRelativeTransform _cube))
  (bind _returnvalue_2 (* _shiphorizontalmovement (.x _moveshipto)))
  (bind _returnvalue_3 (* (.y _moveshipto) _shipverticalmovement))
  (bind _returnvalue_4 (Math|Vector|MakeVector 0.0 _returnvalue_2 _returnvalue_3))
  (bind (_x _y _z) (Math|Vector|BreakVector (.location _returnvalue)))
  (bind _returnvalue_5 (Class|KismetMathLibrary|GetDirectionVector (.location _returnvalue) _returnvalue_4))
  (bind (_x_2 _y_2 _z_2) (Math|Vector|BreakVector _returnvalue_5))
  ;[1 1 1] Move
  (if (> (+ (Math|Float|Absolute(Float) (- (Math|Float|Absolute(Float) _y) (Math|Float|Absolute(Float) _returnvalue_2))) (Math|Float|Absolute(Float) (- (Math|Float|Absolute(Float) _z) (Math|Float|Absolute(Float) _returnvalue_3)))) 2e+01)
    (Transformation|SetRelativeLocation (Variables|Default|GetCube) (+ (* (Math|Vector|MakeVector _x_2 _y_2 (* (Variables|Default|GetShipVerticalMovementSpeedToHorizontal) _z_2)) (* Delta%20Seconds (Variables|Default|GetShipMovementSpeed))) (.location _returnvalue)) false true)
    (else
      (Transformation|SetRelativeLocation (Variables|Default|GetCube) _returnvalue_4 false true))))

(event Custom|MoveUp
  ;[1 1 1] Set movement target
  (if (<= (.y (Variables|Default|GetMoveShipTo)) 0.0)
    (Variables|Default|SetMoveShipTo (Math|Vector2D|MakeVector2D (.x (Variables|Default|GetMoveShipTo)) (+ (.y (Variables|Default|GetMoveShipTo)) 1.0)))))

(event Custom|MoveDown
  ;[1 1 1] Set movement target
  (if (>= (.y (Variables|Default|GetMoveShipTo)) 0.0)
    (Variables|Default|SetMoveShipTo (Math|Vector2D|MakeVector2D (.x (Variables|Default|GetMoveShipTo)) (- (.y (Variables|Default|GetMoveShipTo)) 1.0)))))

(event Custom|MoveRight
  ;[1 1 1] Set movement target
  (if (<= (.x (Variables|Default|GetMoveShipTo)) 0.0)
    (Variables|Default|SetMoveShipTo (Math|Vector2D|MakeVector2D (+ (.x (Variables|Default|GetMoveShipTo)) 1.0) (.y (Variables|Default|GetMoveShipTo))))))

(event Custom|MoveLeft
  ;[1 1 1] Set movement target
  (if (>= (.x (Variables|Default|GetMoveShipTo)) 0.0)
    (Variables|Default|SetMoveShipTo (Math|Vector2D|MakeVector2D (- (.x (Variables|Default|GetMoveShipTo)) 1.0) (.y (Variables|Default|GetMoveShipTo))))))

(event EventBeginPlay)

(event EventActorBeginOverlap
  (params (OtherActor :type Actor%20Object%20Reference)))

(event EventTick
  (params (DeltaSeconds :type Float%20%28single-precision%29))
  (CallFunction|MoveShip DeltaSeconds))

(event Input|ActionEvents|InputActionMoveDown
  (params (Key :type Key%20Structure :default "AnyKey"))
  ;[1 1 1] Key input
  (:Pressed
    (CallFunction|MoveDown)))

(event Input|ActionEvents|InputActionMoveRight
  (params (Key :type Key%20Structure :default "AnyKey"))
  ;[1 1 1] Key input
  (:Pressed
    (CallFunction|MoveRight)))

(event Input|ActionEvents|InputActionMoveLeft
  (params (Key :type Key%20Structure :default "AnyKey"))
  ;[1 1 1] Key input
  (:Pressed
    (CallFunction|MoveLeft)))

(event Input|ActionEvents|InputActionMoveUp
  (params (Key :type Key%20Structure :default "AnyKey"))
  ;[1 1 1] Key input
  (:Pressed
    (CallFunction|MoveUp)))

(event Input|TouchEvents|InputTouch
  (params (Location :type Vector) (FingerIndex :type ETouchIndex%20Enum))
  (:Pressed
    (Variables|Default|SetTouchDownLocation Location))
  (:Released
    (Variables|Default|SetTouchUpLocation Location)))

(fn ConstructionScript)